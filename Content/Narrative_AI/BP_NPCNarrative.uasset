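; BP_NPCNarrative is a narrative NPC that detects the player through an interaction box and shows an interaction prompt.
; On BeginPlay it binds the box's overlap events.
; When a BP_ThirdPersonCharacter enters, it caches that character, reveals the widget component and registers itself as the character's focused NPC.
; When an actor of the cached character's class leaves, it collapses the widget and clears the focus.
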(event `self.ReceiveBeginPlay`
  (add `PrimitiveComponent.OnComponentBeginOverlap` (`self.BoxCollision_Interaction`) (delegate `OnComponentBeginOverlap_Event`))
  (add `PrimitiveComponent.OnComponentEndOverlap` (`self.BoxCollision_Interaction`) (delegate `OnComponentEndOverlap_Event`)))

(event `OnComponentBeginOverlap_Event`
  (params (OverlappedComponent :type "PrimitiveComponent Object Reference") (OtherActor :type "Actor Object Reference") (OtherComp :type "PrimitiveComponent Object Reference") (OtherBodyIndex :type Integer) (bFromSweep :type Boolean) (SweepResult :type "HitResult Structure (by ref)"))
  (bind _asbp_third_person_character (cast `/Game/ThirdPerson/Blueprints/BP_ThirdPersonCharacter` OtherActor))
  (set `self.PlayerCharacter` _asbp_third_person_character)
  (`Widget.SetVisibility` (`WidgetComponent.GetUserWidgetObject` (`self.InteractionWidget`)) "Visible")
  (`NarrativeAITools_UECharacter.SetFocusedNPC` (`self.PlayerCharacter`) self))

(event `OnComponentEndOverlap_Event`
  (params (OverlappedComponent :type "PrimitiveComponent Object Reference") (OtherActor :type "Actor Object Reference") (OtherComp :type "PrimitiveComponent Object Reference") (OtherBodyIndex :type Integer))
  (if (`GameplayStatics.ObjectIsA` OtherActor (`GameplayStatics.GetObjectClass` (`self.PlayerCharacter`)))
    (`Widget.SetVisibility` (`WidgetComponent.GetUserWidgetObject` (`self.InteractionWidget`)) "Collapsed")
    (`NarrativeAITools_UECharacter.ClearFocusedNPC` (`self.PlayerCharacter`))))

(fn `UserConstructionScript`)